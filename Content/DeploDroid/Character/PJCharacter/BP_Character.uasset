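; Player character with Idle, Melee and Ranged stances switched through Enhanced Input.
; Stance governs movement: only Idle can sprint, Melee slows input while attacking, and Ranged slows it further and shows the cursor.
; Melee runs the parent's base attack, with NotifyAttack damaging health components overlapping the attack collision, while Ranged turns toward the cursor hit point and spawns a moving actor.
; The health component's death event destroys the character.
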(event `self.ReceiveBeginPlay`
  ;[1 1 1] Controladores
  (`parent.ReceiveBeginPlay`)
  (bind _asplayer_controller (cast `PlayerController` (`self.GetController`)))
  (`EnhancedInputSubsystemInterface.AddMappingContext` (pcsubsystem `EnhancedInputLocalPlayerSubsystem` _asplayer_controller) "/Game/DeploDroid/Character/Input/IMC_Default.IMC_Default" 0 (struct)))

(event `self.ReceiveActorBeginOverlap`
  (params (OtherActor :type "Actor Object Reference"))
  ;[1 1 1] Sistema de Salud y Daño
)

(event `self.BPC_HealthComponent.DeadCame`
  ;[1 1 1] Sistema de Salud y Daño
  (`self.K2_DestroyActor`))

(event `EnhancedInput|/Game/DeploDroid/Character/Input/Input/IA_Move`
  (params (ActionValue :type "Vector2D Structure") (ElapsedSeconds :type "Float (double-precision)") (TriggeredSeconds :type "Float (double-precision)") (InputAction :type "InputAction Object Reference" :default "/Game/DeploDroid/Character/Input/Input/IA_Move.IA_Move"))
  ;[1 1 1] Movimientos
  (:`Triggered`
    (bind (_x_return _y_return) (`self.Realentizar` (`self.State`) (not (`self.bAtacando?`)) ActionValue_X ActionValue_Y))
    (`self.AddMovementInput` (1.0 0.0 1.0) _x_return)
    (`self.AddMovementInput` (0.0 1.0 0.0) _y_return)))

(event `EnhancedInput|/Game/DeploDroid/Character/Input/Input/IA_Sprint`
  (params (ActionValue :type Boolean) (ElapsedSeconds :type "Float (double-precision)") (TriggeredSeconds :type "Float (double-precision)") (InputAction :type "InputAction Object Reference" :default "/Game/DeploDroid/Character/Input/Input/IA_Sprint.IA_Sprint"))
  ;[1 1 1] Movimientos
  (:`Started`
    (switch `/Game/DeploDroid/Character/E_State` (`self.State`)
      (:`NewEnumerator0`
        (set `CharacterMovementComponent.MaxWalkSpeed` 1200.0 (`self.CharacterMovement`)))
      (:`NewEnumerator1`
        (set `CharacterMovementComponent.MaxWalkSpeed` 600.0 (`self.CharacterMovement`) :!label _label))
      (:`NewEnumerator2`
        (goto _label))))
  (:`Completed`
    (goto _label)))

(event `EnhancedInput|/Game/DeploDroid/Character/Input/Input/IA_Attack`
  (params (ActionValue :type Boolean) (ElapsedSeconds :type "Float (double-precision)") (TriggeredSeconds :type "Float (double-precision)") (InputAction :type "InputAction Object Reference" :default "/Game/DeploDroid/Character/Input/Input/IA_Attack.IA_Attack"))
  ;[1 1 1] Attack
  (:`Triggered`
    (switch `/Game/DeploDroid/Character/E_State` (`self.State`)
      (:`NewEnumerator1`
        (`self.AtaqueBase`))
      (:`NewEnumerator2`
        (`self.Disparar_0`)))))

(event `/Game/DeploDroid/Interfaces/BPI_Player.Notify Attack`
  ;[1 1 1] Attack
  (`self.CheckAttack`))

(event `EnhancedInput|/Game/DeploDroid/Character/Input/Input/IA_StateIdle`
  (params (ActionValue :type Boolean) (ElapsedSeconds :type "Float (double-precision)") (TriggeredSeconds :type "Float (double-precision)") (InputAction :type "InputAction Object Reference" :default "/Game/DeploDroid/Character/Input/Input/IA_StateIdle.IA_StateIdle"))
  ;[1 1 1] States
  (:`Started`
    (set `self.State` "NewEnumerator0")
    (`KismetSystemLibrary.PrintString` "MODO IDLE")
    (set `PlayerController.bShowMouseCursor` false (`GameplayStatics.GetPlayerController` 0))))

(event `EnhancedInput|/Game/DeploDroid/Character/Input/Input/IA_StateMelee`
  (params (ActionValue :type Boolean) (ElapsedSeconds :type "Float (double-precision)") (TriggeredSeconds :type "Float (double-precision)") (InputAction :type "InputAction Object Reference" :default "/Game/DeploDroid/Character/Input/Input/IA_StateMelee.IA_StateMelee"))
  ;[1 1 1] States
  (:`Started`
    (set `self.State` "NewEnumerator1")
    (`KismetSystemLibrary.PrintString` "MODO MELEE")
    (set `PlayerController.bShowMouseCursor` false (`GameplayStatics.GetPlayerController` 0))))

(event `EnhancedInput|/Game/DeploDroid/Character/Input/Input/IA_StateRanged`
  (params (ActionValue :type Boolean) (ElapsedSeconds :type "Float (double-precision)") (TriggeredSeconds :type "Float (double-precision)") (InputAction :type "InputAction Object Reference" :default "/Game/DeploDroid/Character/Input/Input/IA_StateRanged.IA_StateRanged"))
  ;[1 1 1] States
  (:`Started`
    (set `self.State` "NewEnumerator2")
    (`KismetSystemLibrary.PrintString` "MODO RANGED")
    (set `PlayerController.bShowMouseCursor` true (`GameplayStatics.GetPlayerController` 0))))

(fn `AtaqueBase`
  (`parent.AtaqueBase`))

(fn `CheckAttack`
  (for _array_element (`PrimitiveComponent.GetOverlappingActors` (`self.CollisionAttack`) null)
    (`/Game/DeploDroid/Components/BPC_HealthComponent.InflictDamage` (`self.GetComponentByClass` _array_element "/Game/DeploDroid/Components/BPC_HealthComponent.BPC_HealthComponent_C") (`self.Daño_0`))))

(fn `Disparar_0`
  (bind (_returnvalue_roll _returnvalue_pitch _returnvalue_yaw) (`KismetMathLibrary.BreakRotator` (`KismetMathLibrary.FindLookAtRotation` (`KismetMathLibrary.MakeVector` 0.0) (- (`.ImpactPoint` (`GameplayStatics.BreakHitResult` (`PlayerController.GetHitResultUnderCursorByChannel` (`GameplayStatics.GetPlayerController` 0) "TraceTypeQuery1" true))) (`self.K2_GetActorLocation`)))))
  (`self.K2_SetActorRotation` (`KismetMathLibrary.MakeRotator` 0.0 0.0 _returnvalue_yaw))
  (`|SpawnActorFromClass` "/Game/DeploDroid/PropsYBackground/BP_Proyectil.BP_Proyectil_C" (`self.GetTransform`) "Undefined" "MultiplyWithRoot" null 800.0 (`self.GetActorForwardVector`) null))

(fn `Realentizar`
  (params (State :type "/Game/DeploDroid/Character/E_State Enum" :default "NewEnumerator0") (AttackBool :type Boolean) (X :type "Float (double-precision)") (Y :type "Float (double-precision)"))
  (returns (X_return :type "Float (double-precision)") (Y_return :type "Float (double-precision)"))
  (locals (NewLocalVar :type "Float (double-precision)") (NewLocalVar_0 :type "Float (double-precision)") (NewLocalVar_1 :type "Float (double-precision)") (NewLocalVar :type "Float (double-precision)") (NewLocalVar_0 :type "Float (double-precision)") (NewLocalVar :type "Float (double-precision)") (NewLocalVar_0 :type "Float (double-precision)") (NewLocalVar :type "Float (double-precision)") (NewLocalVar_0 :type "Float (double-precision)"))
  (switch `/Game/DeploDroid/Character/E_State` State
    (:`NewEnumerator0`
      _)
    (:`NewEnumerator1`
      (if AttackBool
        _
        (else
          (bind _output_get (set `local.NewLocalVar` (/ X 2.0)))
          (bind _output_get_2 (set `local.NewLocalVar_0` (/ Y 2.0)))
          (return _output_get _output_get_2))))
    (:`NewEnumerator2`
      (bind _output_get_3 (set `local.NewLocalVar` (/ X 4.0)))
      (bind _output_get_4 (set `local.NewLocalVar_0` (/ Y 4.0)))
      (return _output_get_3 _output_get_4)))
  (bind _output_get_5 (set `local.NewLocalVar` X))
  (bind _output_get_6 (set `local.NewLocalVar_0` Y))
  (return _output_get_5 _output_get_6))

(fn `UserConstructionScript`
  (`parent.UserConstructionScript`))