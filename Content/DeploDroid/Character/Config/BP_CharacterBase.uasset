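; Base character Blueprint for DeploDroid that provides shared health, attack and UI hooks.
; On BeginPlay it binds the health component's damage event to UpdateUI, which is empty here, as is the Disparar (shoot) function.
; The inherited AtaqueBase event plays an attack animation override on the Attack slot, using the Atacando flag to block re-triggering until the animation completes.
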(event `self.ReceiveBeginPlay`
  (add `/Game/DeploDroid/Components/BPC_HealthComponent.DamageDone` (`self.BPC_HealthComponent`) (delegate `UpdateUI`)))

(event `UpdateUI`)

(event `AtaqueBase`
  ;[1 1 1] BP_Character Ataque Heredado
  (if (not (`self.bAtacando?`))
    (`PaperZDPlaySlotOverrideAction.PlayAnimationOverrideWithCallbacks` (`PaperZDAnimationComponent.AnimInstance` (`self.AnimationComponent`)) (`self.AnimacionDeAtaque`) "Attack"
      (:`then`
        (set `self.bAtacando?` true))
      (:`OnCompleted`
        (set `self.bAtacando?` false)))))

(fn `Disparar`)

(fn `UserConstructionScript`)