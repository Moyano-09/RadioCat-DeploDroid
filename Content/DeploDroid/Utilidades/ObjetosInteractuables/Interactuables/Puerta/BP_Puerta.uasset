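; BP_Puerta is a door controller that opens a sector by removing a door actor once all its linked consoles are shut down.
; On BeginPlay it records the number of sector consoles and binds to the death event of each one's BPC_HealthComponent.
; Each death increments a counter; when it matches the total, a sound plays at the referenced PuertaConsola actor's location and that actor is destroyed.
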(event `self.ReceiveBeginPlay`
  (set `self.ConsoleQuantity` (`KismetArrayLibrary.Array_Length` (`self.SectorConsole`)))
  (for _array_element _
    (add `/Game/DeploDroid/Components/BPC_HealthComponent.DeadCame` (`self.GetComponentByClass` _array_element "/Game/DeploDroid/Components/BPC_HealthComponent.BPC_HealthComponent_C") (delegate `ConsolesShutDownCounter`))))

(event `ConsolesShutDownCounter`
  (`/Engine/EditorBlueprintResources/StandardMacros.IncrementInt` (`self.ConsoleCounter`)
    (:`  `
      (if (== (`self.ConsoleQuantity`) (`self.ConsoleCounter`))
        (`GameplayStatics.PlaySoundAtLocation` "/Engine/EngineSounds/1kSineTonePing.1kSineTonePing" (`self.K2_GetActorLocation` (`self.PuertaConsola`)) (struct) 5.0 1.0 0.0 null null null null)
        (`self.K2_DestroyActor` (`self.PuertaConsola`))))))

(fn `UserConstructionScript`)