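; BP_Console is an interactable console that shows a green sprite until it is destroyed.
; On BeginPlay it binds to its health component's death event and sets its state to green.
; Death switches the state to red, and SpriteConsoleSetter applies the matching sprite.
; The red case destroys the actor immediately after the sprite swap.
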(event `self.ReceiveBeginPlay`
  (add `/Game/DeploDroid/Components/BPC_HealthComponent.DeadCame` (`self.BPC_HealthComponent`) (delegate `Destroyed`))
  (set `self.ConsoleState` "NewEnumerator0")
  (`self.SpriteConsoleSetter` :!label _label))

(event `Destroyed`
  (set `self.ConsoleState` "NewEnumerator1")
  (goto _label))

(fn `SpriteConsoleSetter`
  (bind _sprite (`self.Sprite`))
  (switch `/Game/DeploDroid/Utilidades/ObjetosInteractuables/Interactuables/Consola/EConsoleState` (`self.ConsoleState`)
    (:`NewEnumerator0`
      (`PaperSpriteComponent.SetSprite` _sprite "/Game/DeploDroid/Utilidades/ObjetosInteractuables/Interactuables/Consola/TilesConsola/ConsolaVerde.ConsolaVerde"))
    (:`NewEnumerator1`
      (`PaperSpriteComponent.SetSprite` _sprite "/Game/DeploDroid/Utilidades/ObjetosInteractuables/Interactuables/Consola/TilesConsola/ConsolaRoja.ConsolaRoja")
      (`self.K2_DestroyActor`))))

(fn `UserConstructionScript`)