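; BP_MuroVariable is a destructible wall that shows intact, damaged or destroyed sprites based on its health.
; BPC_HealthComponent damage events and BeginPlay set WallState by comparing current health to maximum or a fixed damage threshold, while the death event sets the final state.
; SpriteSetter swaps the sprite for each state, plays sounds for damaged states, and removes the Box component on destruction.
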(event `self.BPC_HealthComponent.DamageDone`
  (bind _bpc_healthcomponent (`self.BPC_HealthComponent`))
  (bind _currenthealth (`/Game/DeploDroid/Components/BPC_HealthComponent.CurrentHealth` _bpc_healthcomponent))
  (if (== _currenthealth (`/Game/DeploDroid/Components/BPC_HealthComponent.MaxHealth` _bpc_healthcomponent)) :!label _label
    (set `self.WallState` "NewEnumerator0")
    (`self.SpriteSetter` :!label _label_2)
    (elif (<= _currenthealth 100.0)
      (set `self.WallState` "NewEnumerator1")
      (goto _label_2))))

(event `self.ReceiveBeginPlay`
  (goto _label))

(event `self.BPC_HealthComponent.DeadCame`
  (set `self.WallState` "NewEnumerator2")
  (goto _label_2))

(fn `SpriteSetter`
  (bind _returnvalue (`self.K2_GetActorLocation`))
  (bind _sprite (`self.Sprite`))
  (switch `/Game/DeploDroid/Utilidades/ObjetosInteractuables/Destruibles/Muro/EWallState` (`self.WallState`)
    (:`NewEnumerator0`
      (`PaperSpriteComponent.SetSprite` _sprite "/Game/DeploDroid/Utilidades/ObjetosInteractuables/Destruibles/Muro/SpritesMuro/MuroIntacto.MuroIntacto"))
    (:`NewEnumerator1`
      (`PaperSpriteComponent.SetSprite` _sprite "/Game/DeploDroid/Utilidades/ObjetosInteractuables/Destruibles/Muro/SpritesMuro/MuroDamaged.MuroDamaged")
      (`GameplayStatics.PlaySoundAtLocation` "/Engine/VREditor/Sounds/VR_close.VR_close" _returnvalue (struct) 1.0 1.0 0.0 null null null null))
    (:`NewEnumerator2`
      (`PaperSpriteComponent.SetSprite` _sprite "/Game/DeploDroid/Utilidades/ObjetosInteractuables/Destruibles/Muro/SpritesMuro/MuroDestruido.MuroDestruido")
      (`GameplayStatics.PlaySoundAtLocation` "/Engine/VREditor/Sounds/VR_close.VR_close" _returnvalue (struct) 1.0 1.0 0.0 null null null null)
      (`GameplayStatics.PlaySoundAtLocation` "/Engine/EngineSounds/WhiteNoise.WhiteNoise" _returnvalue (struct) 1.0 1.0 0.0 null null null null)
      (`ActorComponent.K2_DestroyComponent` (`self.Box`)))))

(fn `UserConstructionScript`)