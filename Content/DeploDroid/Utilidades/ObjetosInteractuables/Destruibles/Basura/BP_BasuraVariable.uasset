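; BP_BasuraVariable is a destructible trash prop with three visual states: intact, fallen and destroyed.
; Its health component's damage and death events set TrashState, with BeginPlay reusing the damage check: intact at full health, fallen at half-health threshold or below.
; TrashSpriteSetter swaps the sprite for the state, plays a sound when fallen or destroyed, and removes the Box component on destruction.
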(event `self.BPC_HealthComponent.DamageDone`
  (bind _bpc_healthcomponent (`self.BPC_HealthComponent`))
  (bind _currenthealth (`/Game/DeploDroid/Components/BPC_HealthComponent.CurrentHealth` _bpc_healthcomponent))
  (if (== _currenthealth (`/Game/DeploDroid/Components/BPC_HealthComponent.MaxHealth` _bpc_healthcomponent)) :!label _label
    (set `self.TrashState` "NewEnumerator0")
    (`self.TrashSpriteSetter` :!label _label_2)
    (elif (<= _currenthealth 50.0)
      (set `self.TrashState` "NewEnumerator1")
      (goto _label_2))))

(event `self.ReceiveBeginPlay`
  (goto _label))

(event `self.BPC_HealthComponent.DeadCame`
  (set `self.TrashState` "NewEnumerator2")
  (goto _label_2))

(fn `TrashSpriteSetter`
  (bind _returnvalue (`self.K2_GetActorLocation`))
  (bind _sprite (`self.Sprite`))
  (switch `/Game/DeploDroid/Utilidades/ObjetosInteractuables/Destruibles/Basura/ETrashState` (`self.TrashState`)
    (:`NewEnumerator0`
      (`PaperSpriteComponent.SetSprite` _sprite "/Game/DeploDroid/Utilidades/ObjetosInteractuables/Destruibles/Basura/TilesBasura/BasuraIntacta.BasuraIntacta"))
    (:`NewEnumerator1`
      (`PaperSpriteComponent.SetSprite` _sprite "/Game/DeploDroid/Utilidades/ObjetosInteractuables/Destruibles/Basura/TilesBasura/BasuraCaida.BasuraCaida")
      (`GameplayStatics.PlaySoundAtLocation` "/Engine/EngineSounds/WhiteNoise.WhiteNoise" _returnvalue (struct) 1.0 1.0 0.0 null null null null))
    (:`NewEnumerator2`
      (`PaperSpriteComponent.SetSprite` _sprite "/Game/DeploDroid/Utilidades/ObjetosInteractuables/Destruibles/Basura/TilesBasura/BasuraDestruida.BasuraDestruida")
      (`GameplayStatics.PlaySoundAtLocation` "/Engine/EngineSounds/WhiteNoise.WhiteNoise" _returnvalue (struct) 1.0 1.0 0.0 null null null null)
      (`ActorComponent.K2_DestroyComponent` (`self.Box`)))))

(fn `UserConstructionScript`
  (`parent.UserConstructionScript`))