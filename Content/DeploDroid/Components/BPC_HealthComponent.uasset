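; BPC_HealthComponent is a health component that tracks current and maximum health for its owner.
; InflictDamage subtracts damage, clamping between zero and the current value, prints the result and fires the DamageDone dispatcher, plus DeadCame when health reaches zero.
; ObtenerDataDeSalud returns current and maximum health to callers.
; It is driven by calls and dispatchers, with no active BeginPlay or Tick logic.
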(fn `InflictDamage`
  (params (`Daño` :type "Float (double-precision)"))
  (bind _output_get (set `self.CurrentHealth` (`KismetMathLibrary.FClamp` (- (`self.CurrentHealth`) `Daño`) 0.0 (`self.CurrentHealth`))))
  (if (== _output_get 0.0)
    (`KismetSystemLibrary.PrintString` (`KismetStringLibrary.Conv_DoubleToString` _output_get))
    (`self.DamageDone`)
    (`self.DeadCame`)
    (else
      (`KismetSystemLibrary.PrintString` (`KismetStringLibrary.Conv_DoubleToString` _output_get))
      (`self.DamageDone`))))

(fn `ObtenerDataDeSalud`
  (returns (SaludActual :type "Float (double-precision)") (SaludMaxima :type "Float (double-precision)"))
  (return (`self.CurrentHealth`) (`self.MaxHealth`)))