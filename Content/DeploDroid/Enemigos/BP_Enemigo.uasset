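; BP_Enemigo is an AI enemy that attacks, shows its health through a widget and is destroyed on death.
; On possession by IA_Enemigo it runs BT_Enemigo; events write the target to the Blackboard and trigger the parent's base attack.
; BPC_HealthComponent supplies health data to WBP_SaludEnemiga, and its death event plays a sound before destroying the actor.
; Range debug spheres and an AIMoveTo test remain disconnected.
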(event `self.UpdateUI`
  ;[1 1 1] HEALTH AND DEATH
  (`self.ActualizarSaludEnemiga`))

(event `/Game/DeploDroid/Interfaces/BPI_Enemigo.SetearObjetivo`
  (params (Objetivo :type "Actor Object Reference"))
  ;[1 1 1] Evento Setear Enemigo/Objetivo (detecta al jugador)
  (`BlackboardComponent.SetValueAsObject` (`AIBlueprintHelperLibrary.GetBlackboard` null) (`self.ObjetivoBBKeyName`) Objetivo))

(event `self.ReceiveBeginPlay`
  ;[1 1 1] HEALTH AND DEATH
  (`parent.ReceiveBeginPlay`)
  (`self.ActualizarSaludEnemiga`))

(event `self.BPC_HealthComponent.DeadCame`
  ;[1 1 1] HEALTH AND DEATH
  (`GameplayStatics.PlaySoundAtLocation` "/Engine/VREditor/Sounds/UI/Dockable_Window_Close.Dockable_Window_Close" (`self.K2_GetActorLocation`) (struct) 1.0 1.0 0.0 null null null null)
  (`self.K2_DestroyActor`))

(event `self.ReceivePossessed`
  (params (NewController :type "Controller Object Reference"))
  ;[1 1 1] ¿Que BT usar?
  (bind _asia_enemigo (cast `/Game/DeploDroid/Enemigos/IA/IA_Enemigo` NewController))
  (`AIController.RunBehaviorTree` _asia_enemigo "/Game/DeploDroid/Enemigos/IA/BT_Enemigo.BT_Enemigo"))

(event `/Game/DeploDroid/Interfaces/BPI_Enemigo.AtaqueEnemigo`
  ;[1 1 1] Ataque Enemigo
  (`self.AtaqueBase`))

(event `self.ReceiveTick`
  (params (DeltaSeconds :type "Float (single-precision)"))
  ;[1 1 1] IA Range Debug Sphere
)

(fn `ActualizarSaludEnemiga`
  (bind _aswbp_salud_enemiga (cast `/Game/DeploDroid/Widgets/WBP_SaludEnemiga` (`WidgetComponent.GetUserWidgetObject` (`self.Widget`))))
  (bind (_saludactual _saludmaxima) (`/Game/DeploDroid/Components/BPC_HealthComponent.ObtenerDataDeSalud` (`self.BPC_HealthComponent`)))
  (`/Game/DeploDroid/Widgets/WBP_SaludEnemiga.ActualizarSaludEnemiga` _aswbp_salud_enemiga _saludactual _saludmaxima))

(fn `AtaqueBase`
  (`parent.AtaqueBase`))

(fn `UserConstructionScript`
  (`parent.UserConstructionScript`))