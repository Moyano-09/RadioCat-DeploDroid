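; Trigger volume actor that assigns the player as target to a set of enemies when the player enters, and clears it on exit.
; Overlap events recognize the player through BPI_Jugador, then loop over the Enemigos array calling the SetearObjetivo interface message with the player or with no target.
; Entry uses the actor-level overlap and exit uses the Box component's; the BPI_Enemigo checks on each enemy are left unconnected.
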(event `self.ReceiveActorBeginOverlap`
  (params (OtherActor :type "Actor Object Reference"))
  ;[1 1 1] Detectar al jugador - Checa por interfaz implementada en BP_Enemigo/Distancia y ejecuta
  (if (`KismetSystemLibrary.DoesImplementInterface` OtherActor "/Game/DeploDroid/Interfaces/BPI_Jugador.BPI_Jugador_C")
    (for _array_element (`self.Enemigos`)
      (message `/Game/DeploDroid/Interfaces/BPI_Enemigo.SetearObjetivo` _array_element OtherActor))))

(event `self.Box.OnComponentEndOverlap`
  (params (OverlappedComponent :type "PrimitiveComponent Object Reference") (OtherActor :type "Actor Object Reference") (OtherComp :type "PrimitiveComponent Object Reference") (OtherBodyIndex :type Integer))
  ;[1 1 1] Salir de la hitbox = Cancelar
  (if (`KismetSystemLibrary.DoesImplementInterface` OtherActor "/Game/DeploDroid/Interfaces/BPI_Jugador.BPI_Jugador_C")
    (for _array_element (`self.Enemigos`)
      (message `/Game/DeploDroid/Interfaces/BPI_Enemigo.SetearObjetivo` _array_element null))))

(fn `UserConstructionScript`)