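; BP_EnemigoADistancia is an AI-controlled ranged enemy that attacks by firing BP_ProyectilBala projectiles.
; On possession it starts a behavior tree on its IA_Enemigo controller, and SetearObjetivo writes the target into the Blackboard.
; AtaqueEnemigo spawns the bullet at the enemy's transform.
; Its health component feeds the WBP_SaludEnemiga widget, and death plays a sound and destroys the actor; debug range and movement-test logic is disconnected.
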(event `self.ReceivePossessed`
  (params (NewController :type "Controller Object Reference"))
  ;[1 1 1] ¿Que BT usar?
  (bind _asia_enemigo (cast `/Game/DeploDroid/Enemigos/IA/IA_Enemigo` NewController))
  (`AIController.RunBehaviorTree` _asia_enemigo null))

(event `/Game/DeploDroid/Interfaces/BPI_Enemigo.SetearObjetivo`
  (params (Objetivo :type "Actor Object Reference"))
  ;[1 1 1] Evento Setear Enemigo/Objetivo (detecta al jugador)
  (`BlackboardComponent.SetValueAsObject` (`AIBlueprintHelperLibrary.GetBlackboard` null) (`self.ObjetivoBBKeyName`) Objetivo))

(event `self.ReceiveTick`
  (params (DeltaSeconds :type "Float (single-precision)"))
  ;[1 1 1] IA Range Debug Sphere
)

(event `self.UpdateUI`
  ;[1 1 1] Health Component & UI
  (`self.ActualizarSaludEnemiga`))

(event `self.ReceiveBeginPlay`
  ;[1 1 1] Health Component & UI
  (`parent.ReceiveBeginPlay`)
  (`self.ActualizarSaludEnemiga`))

(event `self.AtaqueEnemigo`
  ;[1 1 1] Ataque a distancia - Enemigo
  (bind _returnvalue (`|SpawnActorFromClass` "/Game/DeploDroid/Utilidades/Proyectiles/BP_ProyectilBala.BP_ProyectilBala_C" (`self.GetTransform`) "Undefined" "MultiplyWithRoot" null 800.0 0.0 null false null))
  (`PrimitiveComponent.IgnoreActorWhenMoving` (`self.CapsuleComponent`) _returnvalue false))

(event `self.BPC_HealthComponent.DeadCame`
  ;[1 1 1] Health Component & UI
  (`GameplayStatics.PlaySoundAtLocation` "/Engine/VREditor/Sounds/VR_click1.VR_click1" (`self.K2_GetActorLocation`) (struct) 1.0 1.0 0.0 null null null null)
  (`self.K2_DestroyActor`))

(fn `ActualizarSaludEnemiga`
  ;[1 1 1] Salud Enemiga
  (bind _aswbp_salud_enemiga (cast `/Game/DeploDroid/Widgets/WBP_SaludEnemiga` (`WidgetComponent.GetUserWidgetObject` (`self.Widget`))))
  (bind (_saludactual _saludmaxima) (`/Game/DeploDroid/Components/BPC_HealthComponent.ObtenerDataDeSalud` (`self.BPC_HealthComponent`)))
  (`/Game/DeploDroid/Widgets/WBP_SaludEnemiga.ActualizarSaludEnemiga` _aswbp_salud_enemiga _saludactual _saludmaxima))

(fn `AtaqueBase`
  (`parent.AtaqueBase`))

(fn `UserConstructionScript`
  (`parent.UserConstructionScript`))